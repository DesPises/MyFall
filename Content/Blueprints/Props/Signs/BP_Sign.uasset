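; BP_Sign is a sign prop that displays English or Russian text on a TextRender.
; On BeginPlay it applies an optional mesh override, then picks the text by current culture, using a FormatText placeholder for line breaks.
; It also caches key mappings from BP_MyFallGM's settings after a one-tick delay.
; A disconnected debug loop can print their order, noted as used for key hints.
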(event `self.ReceiveBeginPlay`
  (bind _signmeshcomp (`self.SignMeshComp`))
  (`|ExecutionSequence`
    (:`then_0`
      (`/Engine/EditorBlueprintResources/StandardMacros.IsValid` _signmeshcomp
        (:`Is Valid`
          (`StaticMeshComponent.SetStaticMesh` (`self.SignMesh`) _signmeshcomp))))
    (:`then_1`
      (`self.AssignLocalizedText`))
    (:`then_2`
      (`KismetSystemLibrary.DelayUntilNextTick`)
      (bind _asbp_my_fall_gm (cast `/Game/Blueprints/BP_MyFallGM` (`GameplayStatics.GetGameMode`)))
      (bind _output_get (set `self.Key Mappings` (`/Game/Blueprints/SG_Settings.KeyMappings` (`/Game/Blueprints/BP_MyFallGM.As SG Settings` _asbp_my_fall_gm)))))))

(fn `AssignLocalizedText`
  (switch `string` (`KismetInternationalizationLibrary.GetCurrentCulture`)
    (:`en`
      (`TextRenderComponent.K2_SetText` (`self.TextRender`) (`|FormatText` (`self.EnText`) " \n")))
    (:`ru`
      (`TextRenderComponent.K2_SetText` (`self.TextRender`) (`|FormatText` (`self.RuText`) " \n")))))

(fn `UserConstructionScript`)