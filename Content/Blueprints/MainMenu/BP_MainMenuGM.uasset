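; Game mode for the main menu that sets UI-only input with a visible cursor and restores saved player settings on BeginPlay.
; If the SG_Settings save slot exists, it loads it, applies music and SFX volumes through sound mix class overrides, pushes the mix and sets the saved language culture.
; A separate AddCoin function increments Score and prints it, with no caller in this Blueprint.
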(event `self.ReceiveBeginPlay`
  (bind _returnvalue (`GameplayStatics.GetPlayerController` 0))
  (`WidgetBlueprintLibrary.SetInputMode_UIOnlyEx` _returnvalue null)
  (set `PlayerController.bShowMouseCursor` true _returnvalue)
  (bind _returnvalue_2 (`GameplayStatics.DoesSaveGameExist` "SG_Settings"))
  (if _returnvalue_2
    (bind _returnvalue_3 (`GameplayStatics.LoadGameFromSlot` "SG_Settings"))
    (bind _output_get (set `self.SG_Settings` _returnvalue_3))
    (bind _assg_settings (cast `/Game/Blueprints/SG_Settings` _output_get))
    (`GameplayStatics.SetSoundMixClassOverride` "/Game/Audio/GameSoundMix.GameSoundMix" "/Game/Audio/MusicSoundClass.MusicSoundClass" (`/Game/Blueprints/SG_Settings.MusicVolume` _assg_settings))
    (`GameplayStatics.SetSoundMixClassOverride` "/Game/Audio/GameSoundMix.GameSoundMix" "/Game/Audio/SFXSoundClass.SFXSoundClass" (`/Game/Blueprints/SG_Settings.SFXVolume` _assg_settings))
    (`GameplayStatics.PushSoundMixModifier` "/Game/Audio/GameSoundMix.GameSoundMix")
    (`KismetInternationalizationLibrary.SetCurrentCulture` (`/Game/Blueprints/SG_Settings.Language` _assg_settings))))

(fn `AddCoin`
  (bind _result (`/Engine/EditorBlueprintResources/StandardMacros.IncrementInt` (`self.Score`))
    (:`  `
      (`KismetSystemLibrary.PrintString` (`KismetStringLibrary.Conv_IntToString` _result)))))

(fn `UserConstructionScript`)