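; BP_MyFallPlayerController is the player controller that toggles the pause menu from the IA_Pause input.
; Pausing creates UI_PauseMenu and freezes the game, with input mode switches delegated to the cached BP_MyFallGM game mode.
; Unpausing calls RemoveMenuWidgets, which closes any pause, settings and key binding widgets.
; Before closing key bindings, it reloads mappings from the SG_Settings save slot, discarding unsaved changes.
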(event `self.ReceiveBeginPlay`
  ;[1 1 1] Defaults
  (bind _asbp_my_fall_gm (cast `/Game/Blueprints/BP_MyFallGM` (`GameplayStatics.GetGameMode`)))
  (set `self.As BP My Fall GM` _asbp_my_fall_gm))

(event `EnhancedInput|/Game/Input/IA_Pause`
  (params (ActionValue :type Boolean) (ElapsedSeconds :type "Float (double-precision)") (TriggeredSeconds :type "Float (double-precision)") (InputAction :type "InputAction Object Reference" :default "/Game/Input/IA_Pause.IA_Pause"))
  ;[1 1 1] Pause
  (:`Started`
    (bind _as_bp_my_fall_gm (`self.As BP My Fall GM`)
      (:`then`
        (if (`GameplayStatics.IsGamePaused`)
          (`GameplayStatics.SetGamePaused` false)
          (`/Game/Blueprints/BP_MyFallGM.InputModeGame` _as_bp_my_fall_gm)
          (`|ExecutionSequence`
            (:`then_0`
              (bind _pausewidget (`self.PauseWidget`)
                (:`then`
                  (`Widget.RemoveFromParent` _pausewidget))
                (:`else`)))
            (:`then_1`
              (bind _settingswidget (`self.SettingsWidget`)
                (:`then`
                  (`Widget.RemoveFromParent` _settingswidget))
                (:`else`)))
            (:`then_2`
              (bind _keybindingswidget (`self.KeyBindingsWidget`)
                (:`then`
                  (bind _returnvalue (`GameplayStatics.LoadGameFromSlot` "SG_Settings"))
                  (bind _assg_settings (cast `/Game/Blueprints/SG_Settings` _returnvalue))
                  (`/Game/Blueprints/UI/UI_KeyBindings.RefreshMappings` _keybindingswidget (`/Game/Blueprints/SG_Settings.KeyMappings` _assg_settings))
                  (`Widget.RemoveFromParent` _keybindingswidget))
                (:`else`))))
          (else
            (`/Game/Blueprints/BP_MyFallGM.InputModeUI` _as_bp_my_fall_gm)
            (bind _returnvalue_2 (`|CreateWidget` "/Game/Blueprints/UI/UI_PauseMenu.UI_PauseMenu_C"))
            (bind _output_get (set `self.PauseWidget` _returnvalue_2))
            (`UserWidget.AddToViewport` _output_get 0)
            (`GameplayStatics.SetGamePaused` true))))
      (:`else`))))

(fn `UserConstructionScript`)