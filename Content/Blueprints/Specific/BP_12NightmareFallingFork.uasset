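; BP_12NightmareFallingFork is a fork prop that falls shortly after the player hits it, then resets itself.
; It stores its starting location and rotation at BeginPlay, and a hit from a Player-tagged actor enables physics on the fork mesh after a brief delay.
; Tick watches the actor's height and, below a fixed world Z, restores the stored transform and switches physics off.
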(event `self.ReceiveBeginPlay`
  (bind (_returnvalue_location _returnvalue_rotation) (`KismetMathLibrary.BreakTransform` (`self.GetTransform`)))
  (set `self.DefaultLocation` _returnvalue_location)
  (set `self.DefaultRotation` _returnvalue_rotation))

(event `self.ForkMesh.OnComponentHit`
  (params (HitComponent :type "PrimitiveComponent Object Reference") (OtherActor :type "Actor Object Reference") (OtherComp :type "PrimitiveComponent Object Reference") (NormalImpulse :type "Vector Structure") (Hit :type "HitResult Structure (by ref)"))
  (if (`self.ActorHasTag` OtherActor "Player")
    (`KismetSystemLibrary.Delay` 0.15)
    (`PrimitiveComponent.SetSimulatePhysics` (`self.ForkMesh`) true)))

(event `self.ReceiveTick`
  (params (DeltaSeconds :type "Float (single-precision)"))
  (bind (_returnvalue_x _returnvalue_y _returnvalue_z) (`KismetMathLibrary.BreakVector` (`self.K2_GetActorLocation`)))
  (if (< _returnvalue_z 550.0)
    (`self.K2_SetActorLocationAndRotation` (`self.DefaultLocation`) (`self.DefaultRotation`))
    (`PrimitiveComponent.SetSimulatePhysics` (`self.ForkMesh`) false)))

(fn `UserConstructionScript`)