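; BP_Door is a level door that opens when puzzle buttons, set traps or both meet the requirement of its LevelType.
; On BeginPlay it counts and binds to every BP_Button and hooks BP_Boris's interact event to count set traps.
; A timeline rotates the mesh's yaw to open and reverses when a button release drops the pushed count below the total, regardless of LevelType.
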(event `self.ReceiveBeginPlay`
  ;[1 1 1] Count activated buttons
  (bind _outactors (`GameplayStatics.GetAllActorsOfClass` "/Game/Blueprints/Props/BP_Button.BP_Button_C"))
  (set `self.ButtonsOnLevel` (`KismetArrayLibrary.Array_Length` _outactors))
  (add `/Game/Blueprints/Props/BP_Button.ButtonPressed` _outactors (delegate `OnButtonPressed`))
  (add `/Game/Blueprints/Props/BP_Button.ButtonReleased` _outactors (delegate `OnButtonReleased`))
  ;[1 1 1] Count activated traps
  (bind _asbp_boris (cast `/Game/Blueprints/Player/BP_Boris` (`GameplayStatics.GetPlayerCharacter` 0)))
  (add `/Game/Blueprints/Player/BP_Boris.Interact` _asbp_boris (delegate `CountSetTraps`)))

(event `CountSetTraps`
  ;[1 1 1] Count activated traps
  (switch `/Game/Blueprints/Player/Interactibles` (`/Game/Blueprints/Player/BP_Boris.AvailableInteractible` (stale `self.ReceiveBeginPlay` _asbp_boris))
    (:`NewEnumerator0`
      (bind _result (`/Engine/EditorBlueprintResources/StandardMacros.IncrementInt` (`self.SetTrapsCounter`))
        (:`  `
          (if (>= _result (`self.TrapsRequiredToWin`))
            (set `self.TrapsSet` true)
            (switch `/Game/Blueprints/Props/LevelType` (`self.LevelType`)
              (:`NewEnumerator0`
                (`self.OpenDoor` :!label _label))
              (:`NewEnumerator2`
                (if (`self.PuzzleSolved`)
                  (goto _label))))))))))

(event `OnButtonPressed`
  ;[1 1 1] Count activated buttons
  (bind _result (`/Engine/EditorBlueprintResources/StandardMacros.IncrementInt` (`self.ButtonsPushed`))
    (:`  `
      (if (>= _result (`self.ButtonsOnLevel`))
        (set `self.PuzzleSolved` true)
        (switch `/Game/Blueprints/Props/LevelType` (`self.LevelType`)
          (:`NewEnumerator1`
            (`self.OpenDoor` :!label _label_2))
          (:`NewEnumerator2`
            (if (`self.TrapsSet`)
              (goto _label_2))))))))

(event `OnButtonReleased`
  ;[1 1 1] Count activated buttons
  (bind _result (`/Engine/EditorBlueprintResources/StandardMacros.DecrementInt` (`self.ButtonsPushed`))
    (:`  `
      (if (< _result (`self.ButtonsOnLevel`))
        (`self.CloseDoor`)
        (set `self.PuzzleSolved` false)))))

(event `OpenDoor`
  ;[1 1 1] Open/Close door events
  (bind (_direction _zrotation) (`Timeline|DoorOpen` :!label _label_3)
    (:`Update`
      (`SceneComponent.K2_SetRelativeRotation` (`self.DoorMesh`) (`KismetMathLibrary.MakeRotator` 0.0 0.0 _zrotation) false false))))

(event `CloseDoor`
  ;[1 1 1] Open/Close door events
  (goto _label_3 :!via `Reverse`))

(fn `UserConstructionScript`)