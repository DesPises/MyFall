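; Trap Blueprint for small glass balls that makes the player character fall when triggered.
; It extends a parent that supplies the trigger event, overlapped actor and construction logic.
; For a Player-tagged BP_Boris it calls FallAsRagdoll, then disables the trigger area's collision, with no re-enable in this Blueprint.
; An Enemy tag check exists but has no effect.
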(event `self.TriggerOnPlayer`
  (bind _triggeroverlappedactor (`self.TriggerOverlappedActor`))
  (if (`self.ActorHasTag` _triggeroverlappedactor "Player")
    (bind _asbp_boris (cast `/Game/Blueprints/Player/BP_Boris` _triggeroverlappedactor))
    (`/Game/Blueprints/Player/BP_Boris.FallAsRagdoll` _asbp_boris)
    (`PrimitiveComponent.SetCollisionEnabled` (`self.TriggerArea`) "NoCollision")
    (elif (`self.ActorHasTag` _triggeroverlappedactor "Enemy")
      _)))

(fn `UserConstructionScript`
  (`parent.UserConstructionScript`))