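; BP_HidingSpot is a base hiding spot that lets the player character, BP_Boris, interact while inside its InteractionZone.
; Entering the zone sets Boris's available interactible and hideout reference and binds his interact event to OnInteract.
; OnInteract calls OnHide, an empty abstract function intended for overrides.
; Leaving the zone updates the interactible, clears the reference and unbinds the event, unless Boris is hiding.
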(event `self.InteractionZone.OnComponentBeginOverlap`
  (params (OverlappedComponent :type "PrimitiveComponent Object Reference") (OtherActor :type "Actor Object Reference") (OtherComp :type "PrimitiveComponent Object Reference") (OtherBodyIndex :type Integer) (bFromSweep :type Boolean) (SweepResult :type "HitResult Structure (by ref)"))
  ;[1 1 1] Check if player is in interaction zone
  (if (== OtherActor (`GameplayStatics.GetPlayerCharacter` 0))
    (bind _asbp_boris (cast `/Game/Blueprints/Player/BP_Boris` OtherActor))
    (set `/Game/Blueprints/Player/BP_Boris.AvailableInteractible` "NewEnumerator1" _asbp_boris)
    (set `/Game/Blueprints/Player/BP_Boris.HideoutRef` self _asbp_boris)
    (add `/Game/Blueprints/Player/BP_Boris.Interact` _asbp_boris (delegate `OnInteract`))))

(event `OnInteract`
  ;[1 1 1] Check if player is in interaction zone
  (`self.OnHide`) ; Abstract function
)

(event `self.InteractionZone.OnComponentEndOverlap`
  (params (OverlappedComponent :type "PrimitiveComponent Object Reference") (OtherActor :type "Actor Object Reference") (OtherComp :type "PrimitiveComponent Object Reference") (OtherBodyIndex :type Integer))
  ;[1 1 1] Check if player is in interaction zone
  (if (== (`GameplayStatics.GetPlayerCharacter` 0) OtherActor)
    (bind _asbp_boris (cast `/Game/Blueprints/Player/BP_Boris` OtherActor))
    (if (not (`/Game/Blueprints/Player/BP_Boris.IsHiding` _asbp_boris))
      (set `/Game/Blueprints/Player/BP_Boris.AvailableInteractible` "NewEnumerator2" _asbp_boris)
      (set `/Game/Blueprints/Player/BP_Boris.HideoutRef` null _asbp_boris)
      (remove `/Game/Blueprints/Player/BP_Boris.Interact` _asbp_boris (delegate `OnInteract`)))))

(fn `OnHide`)

(fn `UserConstructionScript`)