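; Behavior tree task that sends an enemy to the last seen player location stored in the blackboard.
; It sets the pawn's alert state, then runs AIMoveTo toward the LastSeenPlayerLocation key.
; On arrival it clears that key, snaps the pawn's yaw toward the player's current position for a more natural chase, and succeeds; a failed move fails the task.
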(event `self.ReceiveExecuteAI`
  (params (OwnerController :type "AIController Object Reference") (ControlledPawn :type "Pawn Object Reference"))
  (bind _controlled_pawn (`self.Controlled Pawn`))
  (bind _returnvalue (`AIBlueprintHelperLibrary.GetBlackboard` (`self.Controlled Pawn`)))
  (bind (_returnvalue_roll _returnvalue_pitch _returnvalue_yaw) (`KismetMathLibrary.BreakRotator` (`KismetMathLibrary.FindLookAtRotation` (`Actor.K2_GetActorLocation` _controlled_pawn) (`Actor.K2_GetActorLocation` (`GameplayStatics.GetPlayerCharacter` 0)))))
  (bind _output_get (set `self.Controlled Pawn` ControlledPawn))
  (message `/Game/Blueprints/Enemies/BPI_Alert.SetAlertState` _output_get "NewEnumerator1")
  (`|AIMoveTo` (`self.Controlled Pawn`) (`BlackboardComponent.GetValueAsVector` _returnvalue "LastSeenPlayerLocation") null
    (:`OnSuccess`
      (`BlackboardComponent.ClearValue` _returnvalue "LastSeenPlayerLocation")
      ;[1 1 1] Look towards the player to make chasing more natural
      (`Actor.K2_SetActorRotation` _controlled_pawn (`KismetMathLibrary.MakeRotator` 0.0 0.0 _returnvalue_yaw) true)
      (`self.FinishExecute` true))
    (:`OnFail`
      (`self.FinishExecute` false))))