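; BP_LaunchPadTrap is a child trap that ragdolls the player and launches them upward with a spine-bone impulse when triggered.
; A timeline raises the pad mesh, then reverses it once, using a DoOnce to stop Finished from looping.
; The construction script adds a red pad part to the parent's trap meshes.
; Deactivation clears the active flag, then after a short delay enables the indicator and disables those meshes.
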(event `self.TriggerOnPlayer`
  (bind _playerref (`self.PlayerRef`))
  ;[1 1 1] Trigger
  (set `self.IsActive` false)
  (`/Engine/EditorBlueprintResources/StandardMacros.IsValid` _playerref
    (:`Is Valid`
      (`/Game/Blueprints/Player/BP_Boris.FallAsRagdoll` _playerref)
      (`PrimitiveComponent.AddImpulse` (`Character.Mesh` _playerref) (0.0 0.0 50000.0) "DEF-spine_004" false)
      (`|ExecutionSequence`
        (:`then_0`
          (bind (_direction _alpha) (`Timeline|Animation` :!via `PlayFromStart` :!label _label)
            (:`Update`
              (`SceneComponent.K2_SetRelativeLocation` (`self.TrapMesh`) (`KismetMathLibrary.MakeVector` 0.0 0.0 (`KismetMathLibrary.Lerp` -3.5 20.0 _alpha)) false false))
            (:`Finished`
              (`/Engine/EditorBlueprintResources/StandardMacros.DoOnce` false :!label _label_2
                (:`Completed`
                  (goto _label :!via `ReverseFromEnd`))))))
        (:`then_1`
          (goto _label_2 :!via `Reset`))))))

(event `self.Deactivate`
  ;[1 1 1] Deactivate override
  (set `self.IsActive` false)
  (`KismetSystemLibrary.Delay` 1.0)
  (`self.EnableIndincator`)
  (`self.DisableTrapMeshes`))

(fn `UserConstructionScript`
  (`parent.UserConstructionScript`)
  (bind _returnvalue (`AddComponent|NODE_AddStaticMeshComponent-0` :`RelativeTransform` (`KismetMathLibrary.MakeTransform` (0.0 0.0 -4.5) (struct) (1.3 1.3 1.3))))
  (`StaticMeshComponent.SetStaticMesh` _returnvalue "/Game/3D/Traps/Pad/PadPart.PadPart")
  (`PrimitiveComponent.SetMaterial` _returnvalue 0 "/Game/3D/Traps/Pad/M_Red_Inst.M_Red_Inst")
  (`KismetArrayLibrary.Array_Add` (`self.TrapMeshes`) _returnvalue))