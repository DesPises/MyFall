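; Behavior tree task that sends a BP_Enemy along its PatrolLocations in a loop, setting its patrol flags and alert state message.
; AIMoveTo heads to the current location while the wrapping index advances as soon as the move is issued, not on arrival.
; On success it restores default rotation for a single-point route or waits between points, then finishes.
; A failed cast, empty route or failed move never calls FinishExecute.
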(event `self.ReceiveExecuteAI`
  (params (OwnerController :type "AIController Object Reference") (ControlledPawn :type "Pawn Object Reference"))
  (bind _asbp_enemy (cast `/Game/Blueprints/Enemies/BP_Enemy` ControlledPawn))
  (set `/Game/Blueprints/Enemies/BP_Enemy.IsPatrolling` true _asbp_enemy)
  (set `/Game/Blueprints/Enemies/BP_Enemy.IsChasing` false _asbp_enemy)
  (if (> (`KismetArrayLibrary.Array_Length` (`/Game/Blueprints/Enemies/BP_Enemy.PatrolLocations` _asbp_enemy)) 0)
    (message `/Game/Blueprints/Enemies/AlertInterface.SetAlertState` _asbp_enemy "NewEnumerator0")
    (`|AIMoveTo` ControlledPawn (`|GetArrayItem` (`/Game/Blueprints/Enemies/BP_Enemy.PatrolLocations` _asbp_enemy) (`/Game/Blueprints/Enemies/BP_Enemy.CurrentLocationID` _asbp_enemy)) null
      (:`then`
        (if (> (`KismetArrayLibrary.Array_Length` (`/Game/Blueprints/Enemies/BP_Enemy.PatrolLocations` _asbp_enemy)) (+ (`/Game/Blueprints/Enemies/BP_Enemy.CurrentLocationID` _asbp_enemy) 1))
          (`/Engine/EditorBlueprintResources/StandardMacros.IncrementInt` (`/Game/Blueprints/Enemies/BP_Enemy.CurrentLocationID` _asbp_enemy))
          (else
            (set `/Game/Blueprints/Enemies/BP_Enemy.CurrentLocationID` 0 _asbp_enemy))))
      (:`OnSuccess`
        (if (== (`KismetArrayLibrary.Array_Length` (`/Game/Blueprints/Enemies/BP_Enemy.PatrolLocations` _asbp_enemy)) 1)
          (`Actor.K2_SetActorRotation` ControlledPawn (`/Game/Blueprints/Enemies/BP_Enemy.DefaultRotation` _asbp_enemy) false)
          (else
            (`KismetSystemLibrary.Delay` (`/Game/Blueprints/Enemies/BP_Enemy.DelayBetweenPatrolling` _asbp_enemy))))
        (`self.FinishExecute` true)))))