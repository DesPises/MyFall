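; Hint sign that tells the player which key performs a double jump mid-air.
; On BeginPlay it searches the key mappings for the IA Jump entry and takes that key's long display name.
; It inserts the name into English and Russian hint texts, then calls AssignLocalizedText to apply them.
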(event `self.ReceiveBeginPlay`
  (bind _jumpkeyname (`self.JumpKeyName`))
  (`parent.ReceiveBeginPlay`)
  (for _array_element (`self.Key Mappings`)
    (bind (_playermappableoptions _triggers _modifiers _action _key) (break `EnhancedActionKeyMapping` _array_element))
    (switch `string` (`KismetStringLibrary.Conv_NameToString` (`.Name` (break `PlayerMappableKeyOptions` _playermappableoptions)))
      (:`IAJump`
        (set `self.JumpKeyName` (`KismetTextLibrary.Conv_TextToString` (`KismetInputLibrary.Key_GetDisplayName` _key))))))
  (set `self.EnText` (`|FormatText` "Press {Space} \nmid-air to perform \nsecond jump" _jumpkeyname))
  (set `self.RuText` (`|FormatText` "Нажми {Space}, \nв воздухе, чтобы \nотпрыгнуть" _jumpkeyname))
  (`self.AssignLocalizedText`))

(fn `UserConstructionScript`
  (`parent.UserConstructionScript`))