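; BP_SmallObject is a small prop Blueprint that detects when it clips into other things while the player character, BP_Boris, is holding it.
; A box collision's begin overlap sets GrabbedObjectIsClipping on BP_Boris if this object is the grabbed one, ignoring overlaps with the player.
; Any end overlap clears the flag while the object is held, without checking which actor left or whether other overlaps remain.
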(event `self.BoxCollision_ToPreventClipping.OnComponentBeginOverlap`
  (params (OverlappedComponent :type "PrimitiveComponent Object Reference") (OtherActor :type "Actor Object Reference") (OtherComp :type "PrimitiveComponent Object Reference") (OtherBodyIndex :type Integer) (bFromSweep :type Boolean) (SweepResult :type "HitResult Structure (by ref)"))
  (bind _returnvalue (`GameplayStatics.GetPlayerCharacter` 0))
  ;[1 1 1] Prevent clipping while grabbed by player
  (if (!= OtherActor _returnvalue)
    (bind _asbp_boris (cast `/Game/Blueprints/Player/BP_Boris` _returnvalue))
    (if (== (`/Game/Blueprints/Player/BP_Boris.GrabbedObject` _asbp_boris) self)
      (set `/Game/Blueprints/Player/BP_Boris.GrabbedObjectIsClipping` true _asbp_boris))))

(event `self.BoxCollision_ToPreventClipping.OnComponentEndOverlap`
  (params (OverlappedComponent :type "PrimitiveComponent Object Reference") (OtherActor :type "Actor Object Reference") (OtherComp :type "PrimitiveComponent Object Reference") (OtherBodyIndex :type Integer))
  ;[1 1 1] Prevent clipping while grabbed by player
  (bind _asbp_boris (cast `/Game/Blueprints/Player/BP_Boris` (`GameplayStatics.GetPlayerCharacter` 0)))
  (if (== (`/Game/Blueprints/Player/BP_Boris.GrabbedObject` _asbp_boris) self)
    (set `/Game/Blueprints/Player/BP_Boris.GrabbedObjectIsClipping` false _asbp_boris)))

(fn `UserConstructionScript`)