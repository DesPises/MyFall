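; Enemy AI controller that runs the BT_Enemy behavior tree and tracks the player character BP_Boris.
; AI perception updates write SeesPlayer to the blackboard and, when BP_Boris is lost, store the last seen location.
; It binds to the player's hide and unhide events on BeginPlay to keep the PlayerIsHiding blackboard key in sync.
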(event `self.ReceiveBeginPlay`
  (`self.RunBehaviorTree` "/Game/Blueprints/Enemies/BT_Enemy.BT_Enemy")
  (bind _asbp_boris (cast `/Game/Blueprints/Player/BP_Boris` (`GameplayStatics.GetPlayerCharacter` 0)))
  (add `/Game/Blueprints/Player/BP_Boris.HideD` _asbp_boris (delegate `OnPlayerHide`))
  (add `/Game/Blueprints/Player/BP_Boris.UnhideD` _asbp_boris (delegate `OnPlayerUnhide`)))

(event `OnPlayerHide`
  (`BlackboardComponent.SetValueAsBool` (`AIBlueprintHelperLibrary.GetBlackboard` null) "PlayerIsHiding" true))

(event `OnPlayerUnhide`
  (`BlackboardComponent.SetValueAsBool` (`AIBlueprintHelperLibrary.GetBlackboard` null) "PlayerIsHiding" false))

(event `self.AIPerception.OnTargetPerceptionUpdated`
  (params (Actor :type "Actor Object Reference") (Stimulus :type "AIStimulus Structure"))
  (bind (_age _expirationage _strength _stimuluslocation _receiverlocation _tag _bsuccessfullysensed) (break `AIStimulus` Stimulus))
  ;[1 1 1] On see player
  ;;[1 1 1] Check if sensed actor is BP_Boris
  (cast `/Game/Blueprints/Player/BP_Boris` Actor)
  (if _bsuccessfullysensed
    (bind _output_get (set `self.SeesPlayer` true))
    (`BlackboardComponent.SetValueAsBool` (`AIBlueprintHelperLibrary.GetBlackboard` null) "SeesPlayer" _output_get)
    (else
      (bind _output_get_2 (set `self.LastSeenPlayerLocation` _stimuluslocation))
      (`BlackboardComponent.SetValueAsVector` (`AIBlueprintHelperLibrary.GetBlackboard` null) "LastSeenPlayerLocation" _output_get_2)
      (bind _output_get_3 (set `self.SeesPlayer` false))
      (`BlackboardComponent.SetValueAsBool` (`AIBlueprintHelperLibrary.GetBlackboard` null) "SeesPlayer" _output_get_3))))

(fn `UserConstructionScript`)