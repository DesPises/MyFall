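; Behavior tree task that makes an enemy pawn chase the player.
; It sets the pawn's alert-state message, then checks the blackboard flags for seeing the player and the player not hiding.
; When both hold, it moves to the player character and finishes as successful whether the move succeeds or fails.
; When they do not hold, the task never calls finish.
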(event `self.ReceiveExecuteAI`
  (params (OwnerController :type "AIController Object Reference") (ControlledPawn :type "Pawn Object Reference"))
  (bind _returnvalue (`AIBlueprintHelperLibrary.GetBlackboard` (`self.Controlled Pawn`)))
  (bind _output_get (set `self.Controlled Pawn` ControlledPawn))
  (message `/Game/Blueprints/Enemies/BPI_Alert.SetAlertState` _output_get "NewEnumerator1")
  (if (and (`BlackboardComponent.GetValueAsBool` _returnvalue "SeesPlayer") (not (`BlackboardComponent.GetValueAsBool` _returnvalue "PlayerIsHiding")))
    (`|AIMoveTo` (`self.Controlled Pawn`) (0.0 0.0 0.0) (`GameplayStatics.GetPlayerCharacter` 0)
      (:`OnSuccess`
        _)
      (:`OnFail`
        _))
    (`self.FinishExecute` true)))