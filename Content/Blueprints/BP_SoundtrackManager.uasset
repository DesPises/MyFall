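; BP_SoundtrackManager plays the background music and exposes controls for fading and altering it.
; On BeginPlay it spawns a non-auto-destroying 2D sound from MusicAsset, keeps the audio component and fades it in over a configurable duration.
; NormalPitch, LowPitch and HighPitch shift that component's pitch slightly and set its volume, halved for both altered states.
; FadeMusicOut and StopMusic both fade the track out.
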(event `self.ReceiveBeginPlay`
  (bind _returnvalue (`GameplayStatics.SpawnSound2D` (`self.MusicAsset`) 1.0 1.0 0.0 null false false))
  (bind _output_get (set `self.AudioComponent` _returnvalue))
  (`/Engine/EditorBlueprintResources/StandardMacros.IsValid` _output_get
    (:`Is Valid`
      (`AudioComponent.FadeIn` _output_get (`self.Fade in Duration`) 1.0 0.0 "Linear"))))

(event `FadeMusicOut`
  (`AudioComponent.FadeOut` (`self.AudioComponent`) 1.0 0.0 "Linear"))

(fn `HighPitch`
  (bind _audiocomponent (`self.AudioComponent`))
  (`AudioComponent.SetPitchMultiplier` _audiocomponent 1.01)
  (`AudioComponent.SetVolumeMultiplier` _audiocomponent 0.5))

(fn `LowPitch`
  (bind _audiocomponent (`self.AudioComponent`))
  (`AudioComponent.SetPitchMultiplier` _audiocomponent 0.98)
  (`AudioComponent.SetVolumeMultiplier` _audiocomponent 0.5))

(fn `NormalPitch`
  (bind _audiocomponent (`self.AudioComponent`))
  (`AudioComponent.SetPitchMultiplier` _audiocomponent 1.0)
  (`AudioComponent.SetVolumeMultiplier` _audiocomponent 1.0))

(fn `StopMusic`
  (`AudioComponent.FadeOut` (`self.AudioComponent`) 1.0 0.0 "Linear"))

(fn `UserConstructionScript`)