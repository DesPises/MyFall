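; BP_09StationSequence is a level sequence actor that moves the game to the 10_SpaceShipsStation level once an enemy reaches an armed launch pad trap.
; On BeginPlay it finds the BP_LaunchPadTrap, then polls it on Tick and flags it ready after its activation delay.
; An Enemy-tagged actor overlapping the Box while that flag is set triggers a one-shot, delayed level load.
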(event `self.ReceiveBeginPlay`
  (bind _returnvalue (`GameplayStatics.GetActorOfClass` "/Game/Blueprints/Traps/BP_LaunchPadTrap.BP_LaunchPadTrap_C"))
  (set `self.PadTrap` _returnvalue))

(event `self.Box.OnComponentBeginOverlap`
  (params (OverlappedComponent :type "PrimitiveComponent Object Reference") (OtherActor :type "Actor Object Reference") (OtherComp :type "PrimitiveComponent Object Reference") (OtherBodyIndex :type Integer) (bFromSweep :type Boolean) (SweepResult :type "HitResult Structure (by ref)"))
  (if (and (`self.ActorHasTag` OtherActor "Enemy") (`self.TrapIsReadyToDeploy`))
    (`/Engine/EditorBlueprintResources/StandardMacros.DoOnce` false
      (:`Completed`
        (`KismetSystemLibrary.Delay` 7.0)
        (`GameplayStatics.OpenLevelBySoftObjectPtr` "/Game/Levels/10_SpaceShipsStation.10_SpaceShipsStation")))))

(event `self.ReceiveTick`
  (params (DeltaSeconds :type "Float (single-precision)"))
  (if (`/Game/Blueprints/Traps/BP_Trap.IsActive` (`self.PadTrap`))
    (`KismetSystemLibrary.Delay` (`/Game/Blueprints/Traps/BP_Trap.ActivationDelay` (`self.PadTrap`)))
    (set `self.TrapIsReadyToDeploy` true)))

(fn `UserConstructionScript`)