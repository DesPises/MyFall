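; BP_Pie is a spinning pie hazard that traps the BP_Boris character on contact.
; A timeline started at BeginPlay spins the mesh in pitch, and the actor destroys itself after a short delay once it finishes.
; A box overlap with Boris calls GetTrappedByPie with the direction from the pie to the player.
; Any overlap, Boris or not, plays the hit sound and destroys the pie.
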(event `self.ReceiveBeginPlay`
  ;[1 1 1] Rotating animation
  (bind (_direction _alpha) (`Timeline|Rotate`)
    (:`Update`
      (`SceneComponent.K2_SetRelativeRotation` (`self.PieMesh`) (`KismetMathLibrary.MakeRotator` 0.0 (`KismetMathLibrary.Lerp` -90.0 -1000.0 _alpha)) false false))
    (:`Finished`
      (`KismetSystemLibrary.Delay` 3.0)
      (`self.K2_DestroyActor`))))

(event `self.Box.OnComponentBeginOverlap`
  (params (OverlappedComponent :type "PrimitiveComponent Object Reference") (OtherActor :type "Actor Object Reference") (OtherComp :type "PrimitiveComponent Object Reference") (OtherBodyIndex :type Integer) (bFromSweep :type Boolean) (SweepResult :type "HitResult Structure (by ref)"))
  ;[1 1 1] Pie hit
  (bind _asbp_boris (cast `/Game/Blueprints/Player/BP_Boris` OtherActor)
    (:`then`
      (`/Game/Blueprints/Player/BP_Boris.GetTrappedByPie` _asbp_boris (`KismetMathLibrary.Normal` (`KismetMathLibrary.GetDirectionUnitVector` (`self.K2_GetActorLocation`) (`self.K2_GetActorLocation` (`GameplayStatics.GetPlayerCharacter` 0))))))
    (:`CastFailed`
      _))
  (`GameplayStatics.PlaySoundAtLocation` "/Game/Audio/GameplayEffects/Traps/PieHit.PieHit" (`self.K2_GetActorLocation`) (struct) 1.0 1.0 0.0 "/Game/Audio/GameplayEffects/SA_Singing.SA_Singing" null null null)
  (`self.K2_DestroyActor`))

(fn `UserConstructionScript`)