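; BP_Sign_ClimbHint is a sign prop that shows a localized hint for climbing by pressing a key mid-air.
; It extends parent sign logic, waiting one tick after BeginPlay before building English and Russian text with the display name of the first key mapping.
; It then calls AssignLocalizedText to apply the text, and a comment points to BP_Sign for wrong key mappings.
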(event `self.ReceiveBeginPlay`
  (bind _returnvalue (`KismetInputLibrary.Key_GetDisplayName` (`.Key` (break `EnhancedActionKeyMapping` (`|GetArrayItem` (`self.Key Mappings`))))))
  (`parent.ReceiveBeginPlay`)
  (`KismetSystemLibrary.DelayUntilNextTick`)
  (set `self.EnText` (`|FormatText` "Press {Space} \nmid-air to climb" _returnvalue))
  (set `self.RuText` (`|FormatText` "Нажми {Space}, \nв воздухе, чтобы \nзалезть" _returnvalue))
  (`self.AssignLocalizedText`))

(fn `UserConstructionScript`
  (`parent.UserConstructionScript`))