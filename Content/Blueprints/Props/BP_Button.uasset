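; BP_Button is a pressure-plate button prop, activated by overlapping player components or actors tagged Enemy or Small.
; An overlap counter and a DoOnce gate let it press once on the first valid overlap and release only when all objects have left.
; Pressing and releasing fire ButtonPressed or ButtonReleased dispatchers, play a sound, and drive a timeline that lerps the mesh toward its active position or back.
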(event `self.ReceiveBeginPlay`
  (`SceneComponent.K2_SetRelativeLocation` (`self.ButtonMesh`) (0.0 0.0 0.0) false false))

(event `self.BoxCollision.OnComponentBeginOverlap`
  (params (OverlappedComponent :type "PrimitiveComponent Object Reference") (OtherActor :type "Actor Object Reference") (OtherComp :type "PrimitiveComponent Object Reference") (OtherBodyIndex :type Integer) (bFromSweep :type Boolean) (SweepResult :type "HitResult Structure (by ref)"))
  (if (or (`ActorComponent.ComponentHasTag` OtherComp "Player") (`self.ActorHasTag` OtherActor "Enemy") (`self.ActorHasTag` OtherActor "Small"))
    (bind _result (`/Engine/EditorBlueprintResources/StandardMacros.IncrementInt` (`self.CollidingObjects`))
      (:`  `
        (if (> _result 0)
          (`/Engine/EditorBlueprintResources/StandardMacros.DoOnce` false :!label _label
            (:`Completed`
              (`self.ButtonPressed`)
              (`GameplayStatics.PlaySoundAtLocation` "/Game/SFX/GameplayEffects/Puzzle/ButtonPressed.ButtonPressed" (`self.K2_GetActorLocation`) (struct) 1.0 1.0 0.0 "/Game/SFX/Soundtracks/SA_Music.SA_Music" null null null)
              (bind (_direction _pushstate) (`Timeline|PushButtonTL` :!label _label_2)
                (:`Update`
                  (`SceneComponent.K2_SetRelativeLocation` (`self.ButtonMesh`) (`KismetMathLibrary.VLerp` (0.0 0.0 0.0) (`self.ActiveButtonPos`) _pushstate) false false))))))))))

(event `self.BoxCollision.OnComponentEndOverlap`
  (params (OverlappedComponent :type "PrimitiveComponent Object Reference") (OtherActor :type "Actor Object Reference") (OtherComp :type "PrimitiveComponent Object Reference") (OtherBodyIndex :type Integer))
  (if (or (`ActorComponent.ComponentHasTag` OtherComp "Player") (`self.ActorHasTag` OtherActor "Enemy") (`self.ActorHasTag` OtherActor "Small"))
    (bind _output_get (set `self.CollidingObjects` (`KismetMathLibrary.Clamp` (- (`self.CollidingObjects`) 1) 0 555)))
    (if (<= _output_get 0)
      (`|ExecutionSequence`
        (:`then_0`
          (`self.ButtonReleased`)
          (`GameplayStatics.PlaySoundAtLocation` "/Game/SFX/GameplayEffects/Puzzle/ButtonReleased.ButtonReleased" (`self.K2_GetActorLocation`) (struct) 1.0 1.0 0.0 "/Game/SFX/Soundtracks/SA_Music.SA_Music" null null null)
          (goto _label_2 :!via `Reverse`))
        (:`then_1`
          (goto _label :!via `Reset`))))))

(fn `UserConstructionScript`)