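; Game instance that restores saved settings at startup and provides shared keyboard and gamepad menu navigation.
; Init loads the SG_Settings save to apply language and overall scalability preset, falling back to English when no save exists.
; HandleMenu maps a key event to a clamped vertical button index, a stored 0/1 horizontal index, and accept, back and horizontal-input flags, leaving widgets to act on the results.
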(event `self.ReceiveInit`
  ;[1 1 1] Settings
  (bind _returnvalue (`GameplayStatics.DoesSaveGameExist` "SG_Settings"))
  (if _returnvalue
    (bind _returnvalue_2 (`GameplayStatics.LoadGameFromSlot` "SG_Settings"))
    (bind _assg_settings (cast `/Game/Blueprints/SG_Settings` _returnvalue_2))
    (`KismetInternationalizationLibrary.SetCurrentCulture` (`/Game/Blueprints/SG_Settings.Language` _assg_settings) true)
    (bind _returnvalue_3 (`GameUserSettings.GetGameUserSettings`))
    (`GameUserSettings.SetOverallScalabilityLevel` _returnvalue_3 (`/Game/Blueprints/SG_Settings.GraphicsPresetIndex` _assg_settings))
    (`GameUserSettings.ApplySettings` _returnvalue_3 true)
    (else
      (`KismetInternationalizationLibrary.SetCurrentCulture` "en" true))))

(fn `HandleMenu`
  (params (KeyEvent :type "KeyEvent Structure") (SelectedButtonIndex :type Integer) (InteractibleButtons :type Integer))
  (returns (NewSelectedButtonIndex :type Integer) (NewHorizontalIndex :type Integer) (AcceptButton :type Boolean) (BackButton :type Boolean) (HorizontalInput :type Boolean))
  (locals (InteractibleButtonsInWidget :type Integer) (SelectedButtonIndexL :type Integer) (PressedKey :type "Key Structure" :default "None"))
  (bind _pressedkey (`local.PressedKey`))
  (bind _pressedkey_2 (`local.PressedKey`))
  (bind _selectedhorizontalbuttonindex (`self.SelectedHorizontalButtonIndex`))
  (bind _selectedhorizontalbuttonindex_2 (`self.SelectedHorizontalButtonIndex`))
  (bind _selectedbuttonindexl (`local.SelectedButtonIndexL`))
  (bind _selectedbuttonindexl_2 (`local.SelectedButtonIndexL`))
  (bind _pressedkey_3 (`local.PressedKey`))
  (bind _pressedkey_4 (`local.PressedKey`))
  (bind _pressedkey_5 (`local.PressedKey`))
  (bind _pressedkey_6 (`local.PressedKey`))
  (set `local.PressedKey` (`KismetInputLibrary.GetKey` KeyEvent))
  (set `local.SelectedButtonIndexL` SelectedButtonIndex)
  (set `local.InteractibleButtonsInWidget` InteractibleButtons)
  (if (or (== _pressedkey_4 "Down") (== _pressedkey_4 "Gamepad_LeftStick_Down"))
    (bind _result (`/Engine/EditorBlueprintResources/StandardMacros.IncrementInt` (`local.SelectedButtonIndexL`))
      (:`  `
        (return (`KismetMathLibrary.Clamp` _result 0 (- (`local.InteractibleButtonsInWidget`) 1)) _selectedhorizontalbuttonindex false false false)))
    (elif (or (== _pressedkey_5 "Up") (== _pressedkey_5 "Gamepad_LeftStick_Up"))
      (bind _result_2 (`/Engine/EditorBlueprintResources/StandardMacros.DecrementInt` (`local.SelectedButtonIndexL`))
        (:`  `
          (return (`KismetMathLibrary.Clamp` _result_2 0 (- (`local.InteractibleButtonsInWidget`) 1)) _selectedhorizontalbuttonindex false false false)))
      (elif (or (== _pressedkey_6 "Left") (== _pressedkey_6 "Gamepad_LeftStick_Left"))
        (bind _output_get (set `self.SelectedHorizontalButtonIndex` 0))
        (return _selectedbuttonindexl _output_get false false true)
        (elif (or (== _pressedkey "Right") (== _pressedkey "Gamepad_LeftStick_Right"))
          (bind _output_get_2 (set `self.SelectedHorizontalButtonIndex` 1))
          (return _selectedbuttonindexl _output_get_2 false false true)
          (elif (or (== _pressedkey_2 "Enter") (== _pressedkey_2 "Gamepad_FaceButton_Bottom"))
            (return _selectedbuttonindexl_2 _selectedhorizontalbuttonindex_2 true false false)
            (elif (or (== _pressedkey_3 "Escape") (== _pressedkey_3 "Gamepad_FaceButton_Right"))
              (return _selectedbuttonindexl_2 _selectedhorizontalbuttonindex_2 false true false)
              (else
                (return (`local.SelectedButtonIndexL`) (`self.SelectedHorizontalButtonIndex`) false false false)))))))))