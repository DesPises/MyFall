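; Basketball dunk easter egg actor that spawns a hoop ahead of itself and lets the player (BP_Boris) start a dunk.
; On BeginPlay it caches its transform, the dunk end point and the soundtrack manager, while its overlap box binds or unbinds the player's interaction.
; Interacting attaches the ball to the player, disables ball and hoop collision and mutes music.
; Stopping detaches it, lerps it home by timeline and restores collision and volume.
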(event `self.ReceiveBeginPlay`
  (bind (_returnvalue_roll _returnvalue_pitch _returnvalue_yaw) (`KismetMathLibrary.BreakRotator` (`self.K2_GetActorRotation`)))
  ;[1 1 1] Set defaults
  (set `self.DefaultTransform` (`KismetMathLibrary.MakeTransform` (`self.K2_GetActorLocation`) (`self.K2_GetActorRotation`)))
  (bind _returnvalue (`|SpawnActorFromClass` "/Game/Blueprints/Props/BP_BasketballHoop.BP_BasketballHoop_C" (`KismetMathLibrary.MakeTransform` (+ (`self.K2_GetActorLocation`) (* (`self.GetActorForwardVector`) 650.0) (0.0 0.0 -20.0)) (`KismetMathLibrary.MakeRotator` 0.0 0.0 (+ _returnvalue_yaw 180.0))) "AlwaysSpawn" "MultiplyWithRoot" null null))
  (set `self.HoopRef` _returnvalue)
  (`self.SetDunkEndLocation`)
  (bind _returnvalue_2 (`GameplayStatics.GetActorOfClass` "/Game/Blueprints/BP_SoundtrackManager.BP_SoundtrackManager_C"))
  (set `self.SoundtrackManager` _returnvalue_2))

(event `DetachBall`
  (bind _hoopref (`self.HoopRef`))
  (bind (_defaulttransform_location _defaulttransform_rotation) (`KismetMathLibrary.BreakTransform` (`self.DefaultTransform`)))
  ;[1 1 1] Stop dunk
  (`|ExecutionSequence`
    (:`then_0`
      (set `self.IsPerformingDunk` false)
      (bind _asbp_boris (cast `/Game/Blueprints/Player/BP_Boris` (`GameplayStatics.GetPlayerCharacter` 0)))
      (set `/Game/Blueprints/Player/BP_Boris.AvailableInteractible` "NewEnumerator2" _asbp_boris)
      (`self.K2_DetachFromActor` "KeepWorld" "KeepWorld" "KeepWorld")
      (`self.K2_SetActorLocation` (`SceneComponent.K2_GetComponentLocation` (`self.BallMesh`)))
      (`SceneComponent.K2_SetRelativeLocation` (`self.BallMesh`) (0.0 0.0 0.0) false false)
      (bind (_direction _alpha) (`Timeline|GetBallBack` :!via `PlayFromStart`)
        (:`Update`
          (`self.K2_SetActorLocationAndRotation` (`KismetMathLibrary.VLerp` (`self.K2_GetActorLocation`) _defaulttransform_location _alpha) _defaulttransform_rotation))
        (:`Finished`
          (for _array_element (`|MakeArray` (`/Game/Blueprints/Props/BP_BasketballHoop.StaticMesh` _hoopref) (`/Game/Blueprints/Props/BP_BasketballHoop.StaticMesh1` _hoopref) (`/Game/Blueprints/Props/BP_BasketballHoop.StaticMesh2` _hoopref) (`self.BallMesh`))
            (`PrimitiveComponent.SetCollisionEnabled` _array_element "QueryAndPhysics")))))
    (:`then_1`
      (bind _soundtrackmanager (`self.SoundtrackManager`)
        (:`then`
          (`AudioComponent.SetVolumeMultiplier` (`/Game/Blueprints/BP_SoundtrackManager.AudioComponent` _soundtrackmanager) (`self.OldMusicVolume`)))
        (:`else`)))))

(event `self.Box.OnComponentBeginOverlap`
  (params (OverlappedComponent :type "PrimitiveComponent Object Reference") (OtherActor :type "Actor Object Reference") (OtherComp :type "PrimitiveComponent Object Reference") (OtherBodyIndex :type Integer) (bFromSweep :type Boolean) (SweepResult :type "HitResult Structure (by ref)"))
  (if (and (`self.ActorHasTag` OtherActor "Player") (not (`self.IsPerformingDunk`)))
    (bind _asbp_boris (cast `/Game/Blueprints/Player/BP_Boris` OtherActor))
    (set `/Game/Blueprints/Player/BP_Boris.AvailableInteractible` "NewEnumerator3" _asbp_boris)
    (add `/Game/Blueprints/Player/BP_Boris.Interact` _asbp_boris (delegate `AttachBall`))
    (add `/Game/Blueprints/Player/BP_Boris.StopDunk` _asbp_boris (delegate `DetachBall`))
    (set `/Game/Blueprints/Player/BP_Boris.DunkEERef` self _asbp_boris)))

(event `AttachBall`
  (bind _hoopref (`self.HoopRef`))
  ;[1 1 1] Start dunk
  (`|ExecutionSequence`
    (:`then_0`
      (bind _asbp_boris (cast `/Game/Blueprints/Player/BP_Boris` (stale `self.Box.OnComponentBeginOverlap` OtherActor)))
      (set `/Game/Blueprints/Player/BP_Boris.AvailableInteractible` "NewEnumerator2" _asbp_boris)
      (`self.K2_AttachToActor` (stale `self.Box.OnComponentBeginOverlap` OtherActor) "None" "SnapToTarget" "SnapToTarget" "KeepWorld")
      (`self.K2_SetActorRelativeLocation` (0.0 0.0 -72.0))
      (for _array_element (`|MakeArray` (`/Game/Blueprints/Props/BP_BasketballHoop.StaticMesh` _hoopref) (`/Game/Blueprints/Props/BP_BasketballHoop.StaticMesh1` _hoopref) (`/Game/Blueprints/Props/BP_BasketballHoop.StaticMesh2` _hoopref) (`self.BallMesh`))
        (`PrimitiveComponent.SetCollisionEnabled` _array_element "NoCollision")))
    (:`then_1`
      (bind _soundtrackmanager (`self.SoundtrackManager`)
        (:`then`
          (`AudioComponent.SetVolumeMultiplier` (`/Game/Blueprints/BP_SoundtrackManager.AudioComponent` _soundtrackmanager) 0.0))
        (:`else`)))))

(event `self.Box.OnComponentEndOverlap`
  (params (OverlappedComponent :type "PrimitiveComponent Object Reference") (OtherActor :type "Actor Object Reference") (OtherComp :type "PrimitiveComponent Object Reference") (OtherBodyIndex :type Integer))
  (if (and (`self.ActorHasTag` OtherActor "Player") (not (`self.IsPerformingDunk`)))
    (bind _asbp_boris (cast `/Game/Blueprints/Player/BP_Boris` OtherActor))
    (set `/Game/Blueprints/Player/BP_Boris.AvailableInteractible` "NewEnumerator2" _asbp_boris)
    (remove `/Game/Blueprints/Player/BP_Boris.Interact` _asbp_boris (delegate `AttachBall`))))

(fn `GetLookAtZRotation`
  (returns (`Return Value Z (Yaw)` :type "Float (single-precision)"))
  (bind (_returnvalue_roll _returnvalue_pitch _returnvalue_yaw) (`KismetMathLibrary.BreakRotator` (`KismetMathLibrary.FindLookAtRotation` (`self.K2_GetActorLocation` (`GameplayStatics.GetPlayerCharacter` 0)) (`self.K2_GetActorLocation` (`self.HoopRef`)))))
  (return _returnvalue_yaw))

(fn `SetDunkEndLocation`
  (set `self.DunkEndLocation` (+ (`self.K2_GetActorLocation`) (* (`self.GetActorForwardVector`) 500.0) (0.0 0.0 72.0))))

(fn `UserConstructionScript`)