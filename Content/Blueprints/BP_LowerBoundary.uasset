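; BP_LowerBoundary is a trigger volume that returns the player and small objects to safe positions when they overlap its box.
; A tagged player releases any grab and teleports to one of up to two spawn points, picked by comparing Y position to a zone border when there are two.
; Tagged small objects move back to their stored default location with linear velocity cleared.
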(event `self.ReceiveBeginPlay`
  (set `self.CharacterRef` (`GameplayStatics.GetPlayerCharacter` 0)))

(event `self.Box.OnComponentBeginOverlap`
  (params (OverlappedComponent :type "PrimitiveComponent Object Reference") (OtherActor :type "Actor Object Reference") (OtherComp :type "PrimitiveComponent Object Reference") (OtherBodyIndex :type Integer) (bFromSweep :type Boolean) (SweepResult :type "HitResult Structure (by ref)"))
  (bind _characterref (`self.CharacterRef`))
  (bind _spawnpoints (`self.SpawnPoints`))
  (bind (_returnvalue_x _returnvalue_y) (`KismetMathLibrary.BreakVector` (`self.K2_GetActorLocation` (`self.CharacterRef`))))
  (bind _output (`|GetArrayItem` _spawnpoints))
  (bind _output_get (set `self.Other Actor` OtherActor))
  (if (`self.ActorHasTag` _output_get "Player")
    ;[1 1 1] Player
    (bind _asbp_boris (cast `/Game/Blueprints/Player/BP_Boris` (`self.CharacterRef`)))
    (`/Game/Blueprints/Player/BP_Boris.StopGrabbing` _asbp_boris)
    (if (== (`KismetArrayLibrary.Array_Length` _spawnpoints) 1)
      (`self.K2_SetActorLocation` (`self.CharacterRef`) _output false false)
      (elif (> _returnvalue_y (`self.YRespawnZoneBorder`))
        (`self.K2_SetActorLocation` _characterref _output false false)
        (else
          (`self.K2_SetActorLocation` _characterref (`|GetArrayItem` _spawnpoints 1) false false))))
    (elif (`self.ActorHasTag` _output_get "Small")
      ;[1 1 1] Small object
      (bind _asbp_small_object (cast `/Game/Blueprints/Props/SmallObjects/BP_SmallObject` (`self.Other Actor`)))
      (`self.K2_SetActorLocationAndRotation` :`self` (`self.Other Actor`) :`NewLocation` (`/Game/Blueprints/Props/SmallObjects/BP_SmallObject.DefaultLocation` _asbp_small_object))
      (`PrimitiveComponent.SetPhysicsLinearVelocity` (`/Game/Blueprints/Props/SmallObjects/BP_SmallObject.StaticMesh` _asbp_small_object) (0.0 0.0 0.0) false "None"))))

(fn `UserConstructionScript`)