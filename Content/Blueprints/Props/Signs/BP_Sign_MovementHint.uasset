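; Sign prop that shows the player a movement and jump hint using their current key bindings, in English and Russian.
; On BeginPlay it runs the parent sign logic, waits a tick, then formats both texts from display names of KeyMappings entries picked by fixed index.
; It then calls AssignLocalizedText to apply the text, so correct keys depend on the mapping order noted in BP_Sign.
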(event `self.ReceiveBeginPlay`
  (bind _key_mappings (`self.Key Mappings`))
  (bind _returnvalue (`KismetInputLibrary.Key_GetDisplayName` (`.Key` (break `EnhancedActionKeyMapping` (`|GetArrayItem` _key_mappings 6)))))
  (bind _returnvalue_2 (`KismetInputLibrary.Key_GetDisplayName` (`.Key` (break `EnhancedActionKeyMapping` (`|GetArrayItem` _key_mappings)))))
  (bind _returnvalue_3 (`KismetInputLibrary.Key_GetDisplayName` (`.Key` (break `EnhancedActionKeyMapping` (`|GetArrayItem` _key_mappings 3)))))
  (bind _returnvalue_4 (`KismetInputLibrary.Key_GetDisplayName` (`.Key` (break `EnhancedActionKeyMapping` (`|GetArrayItem` _key_mappings 4)))))
  (bind _returnvalue_5 (`KismetInputLibrary.Key_GetDisplayName` (`.Key` (break `EnhancedActionKeyMapping` (`|GetArrayItem` _key_mappings 5)))))
  (`parent.ReceiveBeginPlay`)
  (`KismetSystemLibrary.DelayUntilNextTick`)
  (set `self.EnText` (`|FormatText` "{W}{A}{S}{D} - move \n{Space} - jump" _returnvalue_3 _returnvalue_4 _returnvalue_5 _returnvalue _returnvalue_2))
  (set `self.RuText` (`|FormatText` "{W}{A}{S}{D} - ходить \n{Space} - прыгать" _returnvalue_3 _returnvalue_4 _returnvalue_5 _returnvalue _returnvalue_2))
  (`self.AssignLocalizedText`))

(fn `UserConstructionScript`
  (`parent.UserConstructionScript`))