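; BP_Sign_SwingHint is a sign prop that shows the player which keys to use for swinging.
; One tick after the parent BeginPlay, it formats English and Russian hint strings using key display names read by fixed index from KeyMappings.
; It then calls AssignLocalizedText, with a note pointing to BP_Sign if the key mappings come out wrong.
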(event `self.ReceiveBeginPlay`
  (bind _key_mappings (`self.Key Mappings`))
  (bind _returnvalue (`KismetInputLibrary.Key_GetDisplayName` (`.Key` (break `EnhancedActionKeyMapping` (`|GetArrayItem` _key_mappings 3)))))
  (bind _returnvalue_2 (`KismetInputLibrary.Key_GetDisplayName` (`.Key` (break `EnhancedActionKeyMapping` (`|GetArrayItem` _key_mappings 5)))))
  (`parent.ReceiveBeginPlay`)
  (`KismetSystemLibrary.DelayUntilNextTick`)
  (set `self.EnText` (`|FormatText` "Use {W} or {S} \nto swing" _returnvalue _returnvalue_2))
  (set `self.RuText` (`|FormatText` "Используй  \n{W} или {S}, \nчтобы раскачиваться" _returnvalue _returnvalue_2))
  (`self.AssignLocalizedText`))

(fn `UserConstructionScript`
  (`parent.UserConstructionScript`))