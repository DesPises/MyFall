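; BP_Collectible is a coin bag pickup that bobs, rotates and plays a shiny coin sound in the world.
; Two timelines lerp the mesh's height and yaw, each ping-ponging through a FlipFlop on finish, so the spin reverses after each full turn.
; When the player character overlaps the sphere, it calls PickupMessage on the game mode, stops the sound spawned at BeginPlay and destroys itself.
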(event `self.ReceiveBeginPlay`
  (`|ExecutionSequence`
    (:`then_0`
      (bind (_direction _newtrack_0) (`Timeline|Animation` :!label _label)
        (:`Update`
          (`SceneComponent.K2_SetRelativeLocation` (`self.CoinBagMesh`) (`KismetMathLibrary.MakeVector` 0.0 0.0 (`KismetMathLibrary.Lerp` -30.0 -10.0 _newtrack_0)) false false))
        (:`Finished`
          (`/Engine/EditorBlueprintResources/StandardMacros.FlipFlop`
            (:`A`
              (goto _label :!via `ReverseFromEnd`))
            (:`B`
              (goto _label :!via `PlayFromStart`))))))
    (:`then_1`
      (bind (_direction_2 _newtrack_0_2) (`Timeline|Rotation` :!label _label_2)
        (:`Update`
          (`SceneComponent.K2_SetRelativeRotation` (`self.CoinBagMesh`) (`KismetMathLibrary.MakeRotator` 0.0 0.0 (`KismetMathLibrary.Lerp` 0.0 360.0 _newtrack_0_2)) false false))
        (:`Finished`
          (`/Engine/EditorBlueprintResources/StandardMacros.FlipFlop`
            (:`A`
              (goto _label_2 :!via `ReverseFromEnd`))
            (:`B`
              (goto _label_2 :!via `PlayFromStart`))))))
    (:`then_2`
      (bind _returnvalue (`GameplayStatics.SpawnSoundAtLocation` "/Game/SFX/GameplayEffects/Puzzle/ShinyCoin.ShinyCoin" (`self.K2_GetActorLocation`) (struct) 1.0 1.0 0.0 "/Game/SFX/GameplayEffects/SA_Effect.SA_Effect" null))
      (set `self.SoundEffect` _returnvalue))))

(event `self.Sphere.OnComponentBeginOverlap`
  (params (OverlappedComponent :type "PrimitiveComponent Object Reference") (OtherActor :type "Actor Object Reference") (OtherComp :type "PrimitiveComponent Object Reference") (OtherBodyIndex :type Integer) (bFromSweep :type Boolean) (SweepResult :type "HitResult Structure (by ref)"))
  (if (== OtherActor (`GameplayStatics.GetPlayerCharacter` 0))
    (message `/Game/Blueprints/BPI_Pickup.Pickup` (`GameplayStatics.GetGameMode`))
    (`AudioComponent.Stop` (`self.SoundEffect`))
    (`self.K2_DestroyActor`)))

(fn `UserConstructionScript`)