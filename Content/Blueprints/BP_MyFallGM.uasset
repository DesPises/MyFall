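; Game mode that manages level setup, coin and trap statistics, and level transitions.
; BeginPlay sets game input, caches soundtrack and Boris references, counts coins and inactive traps, applies saved volume and language, and shows the end transition.
; StartLevelTransition fades music, tallies worked traps, optionally plays applause, shows transition and level-end widgets, and disables Boris's movement; OpenNextLevel calls C++.
; Saved key bindings load through a briefly displayed UI_KeyBindings widget as a workaround.
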(event `self.ReceiveBeginPlay`
  (`|ExecutionSequence`
    (:`then_0`
      (`|ExecutionSequence`
        (:`then_0`
          (`self.InputModeGame`)
          (bind _returnvalue (`GameplayStatics.GetActorOfClass` "/Game/Blueprints/BP_SoundtrackManager.BP_SoundtrackManager_C"))
          (set `self.SoundtrackManager` _returnvalue)
          (bind _returnvalue_2 (`GameplayStatics.GetActorOfClass` "/Game/Blueprints/Player/BP_Boris.BP_Boris_C"))
          (set `self.BorisRef` _returnvalue_2)
          (bind _outactors (`GameplayStatics.GetAllActorsOfClass` "/Game/Blueprints/Props/BP_Collectible.BP_Collectible_C"))
          (set `self.CoinsOnLevel` (`KismetArrayLibrary.Array_Length` _outactors))
          (bind _outactors_2 (`GameplayStatics.GetAllActorsOfClass` "/Game/Blueprints/Traps/BP_Trap.BP_Trap_C"))
          (for _array_element _outactors_2
            (if (not (`/Game/Blueprints/Traps/BP_Trap.IsActive` _array_element))
              (`/Engine/EditorBlueprintResources/StandardMacros.IncrementInt` (`self.InitiallyInactiveTrapsOnLevel`)))))
        (:`then_1`
          (bind _returnvalue_3 (`GameplayStatics.DoesSaveGameExist` "SG_Settings"))
          (if _returnvalue_3
            (bind _returnvalue_4 (`GameplayStatics.LoadGameFromSlot` "SG_Settings"))
            (bind _assg_settings (cast `/Game/Blueprints/SG_Settings` _returnvalue_4))
            (bind _output_get (set `self.As SG Settings` _assg_settings))
            (`GameplayStatics.SetSoundMixClassOverride` "/Game/Audio/GameSoundMix.GameSoundMix" "/Game/Audio/MusicSoundClass.MusicSoundClass" (`/Game/Blueprints/SG_Settings.MusicVolume` _output_get) 1.0 0.0)
            (`GameplayStatics.SetSoundMixClassOverride` "/Game/Audio/GameSoundMix.GameSoundMix" "/Game/Audio/SFXSoundClass.SFXSoundClass" (`/Game/Blueprints/SG_Settings.SFXVolume` _output_get) 1.0 0.0)
            (`GameplayStatics.PushSoundMixModifier` "/Game/Audio/GameSoundMix.GameSoundMix")
            (`KismetInternationalizationLibrary.SetCurrentCulture` (`/Game/Blueprints/SG_Settings.Language` _output_get) true)
            (bind _returnvalue_5 (`|CreateWidget` "/Game/Blueprints/UI/UI_KeyBindings.UI_KeyBindings_C"))
            (`UserWidget.AddToViewport` _returnvalue_5 0)
            (`KismetSystemLibrary.DelayUntilNextTick`)
            (`Widget.RemoveFromParent` _returnvalue_5)))))
    (:`then_1`
      ;[1 1 1] End level transition
      ;;[1 1 1] TODO: if any level needs no transition, implement some variable for that
      (if true
        (bind _returnvalue_6 (`|CreateWidget` "/Game/Blueprints/UI/UI_EndTransition.UI_EndTransition_C"))
        (`UserWidget.AddToViewport` _returnvalue_6 0)))))

(event `InputModeUI`
  (bind _returnvalue (`GameplayStatics.GetPlayerController` 0))
  ;[1 1 1] Input mode functions
  (`WidgetBlueprintLibrary.SetInputMode_UIOnlyEx` _returnvalue null)
  (set `PlayerController.bShowMouseCursor` true _returnvalue))

(event `InputModeGame`
  (bind _returnvalue (`GameplayStatics.GetPlayerController` 0))
  ;[1 1 1] Input mode functions
  (`WidgetBlueprintLibrary.SetInputMode_GameOnly` _returnvalue)
  (set `PlayerController.bShowMouseCursor` false _returnvalue))

(event `StartLevelTransition`
  (params (NextLevel :type "World Soft Object Reference") (ApplauseSound :type Boolean :default true))
  (bind _returnvalue (`GameplayStatics.GetPlayerController` 0))
  ;[1 1 1] Start level transition
  (set `self.Next Level` NextLevel)
  (`|ExecutionSequence`
    (:`then_0`
      (bind _soundtrackmanager (`self.SoundtrackManager`)
        (:`then`
          (`/Game/Blueprints/BP_SoundtrackManager.FadeMusicOut` _soundtrackmanager))
        (:`else`)))
    (:`then_1`
      (bind _outactors (`GameplayStatics.GetAllActorsOfClass` "/Game/Blueprints/Traps/BP_Trap.BP_Trap_C"))
      (for _array_element _outactors
        (if (`/Game/Blueprints/Traps/BP_Trap.WorkedOnEnemyAtLeastOnce` _array_element)
          (`/Engine/EditorBlueprintResources/StandardMacros.IncrementInt` (`self.WorkedTraps`)))))
    (:`then_2`
      (if ApplauseSound
        (`GameplayStatics.PlaySound2D` "/Game/Audio/GameplayEffects/Applause/LoudApplouse.LoudApplouse" 1.0 1.0 0.0 null null)))
    (:`then_3`
      (bind _returnvalue_2 (`|CreateWidget` "/Game/Blueprints/UI/UI_BeginTransition.UI_BeginTransition_C" _returnvalue))
      (`UserWidget.AddToViewport` _returnvalue_2 0)
      (bind _returnvalue_3 (`|CreateWidget` "/Game/Blueprints/UI/UI_LevelEnd.UI_LevelEnd_C" _returnvalue))
      (`UserWidget.AddToViewport` _returnvalue_3 0)
      (bind _borisref (`self.BorisRef`)
        (:`then`
          (`/Game/Blueprints/Player/BP_Boris.DisableMovement` _borisref)
          (`KismetSystemLibrary.Delay` 0.5)
          (set `self.WaitingForLevelTransition` true))
        (:`else`)))))

(event `/Game/Blueprints/BPI_Pickup.Pickup`
  ;[1 1 1] Pickup
  (`GameplayStatics.PlaySound2D` "/Game/Audio/GameplayEffects/Puzzle/coindrop.coindrop" 1.0 1.0 0.0 null null)
  (`GameplayStatics.PlaySound2D` "/Game/Audio/GameplayEffects/Applause/Applause_Cue.Applause_Cue" 1.0 1.0 0.0 null null)
  (`self.AddCoin`))

(event `OpenNextLevel`
  (`self.OpenNextLevelCPP` (`self.Next Level`)))

(event `/Game/Blueprints/Traps/BPI_TrapActivation.TrapActivated`
  (`/Engine/EditorBlueprintResources/StandardMacros.IncrementInt` (`self.TrapsActivatedByPlayer`)))

(fn `AddCoin`
  (`/Engine/EditorBlueprintResources/StandardMacros.IncrementInt` (`self.CollectedCoins`)))

(fn `UserConstructionScript`)