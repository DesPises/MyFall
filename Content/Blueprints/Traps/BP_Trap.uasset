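; Base trap that the player arms by interacting and that springs on actors tagged Player or Enemy.
; Interaction area binds OnActivate on BP_Boris; activation shows meshes, hides the indicator and enables the trigger after a delay.
; Springing calls empty TriggerOnPlayer or TriggerOnEnemy hooks, then deactivates for rearming.
; First manual activation notifies BP_Door and BP_MyFallGM; first enemy hit calls TrapWorked.
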(event `self.ReceiveBeginPlay`
  ;[1 1 1] Set player reference
  (bind _asbp_boris (cast `/Game/Blueprints/Player/BP_Boris` (`GameplayStatics.GetPlayerCharacter` 0))
    (:`then`
      (set `self.PlayerRef` _asbp_boris)
      (if (`self.IsActive`)
        (`self.Activate`)
        (set `self.WasActivatedOnce` true)
        (`PrimitiveComponent.SetCollisionEnabled` (`self.TriggerArea`) "QueryOnly")
        (else
          (`self.Deactivate`))))
    (:`CastFailed`
      (`KismetSystemLibrary.PrintString` "Wrong player character"))))

(event `self.InteractionArea.OnComponentBeginOverlap`
  (params (OverlappedComponent :type "PrimitiveComponent Object Reference") (OtherActor :type "Actor Object Reference") (OtherComp :type "PrimitiveComponent Object Reference") (OtherBodyIndex :type Integer) (bFromSweep :type Boolean) (SweepResult :type "HitResult Structure (by ref)"))
  (bind _playerref (`self.PlayerRef`))
  ;[1 1 1] Interaction
  (if (and (== OtherActor (`GameplayStatics.GetPlayerCharacter` 0)) (not (`self.IsActive`)))
    (`/Engine/EditorBlueprintResources/StandardMacros.IsValid` _playerref
      (:`Is Valid`
        (set `/Game/Blueprints/Player/BP_Boris.AvailableInteractible` "NewEnumerator0" _playerref)
        (add `/Game/Blueprints/Player/BP_Boris.Interact` _playerref (delegate `OnActivate`))))))

(event `OnActivate`
  ;[1 1 1] Interaction
  (set `/Game/Blueprints/Player/BP_Boris.AvailableInteractible` "NewEnumerator2" (`self.PlayerRef`))
  (`self.Activate`)
  (`|ExecutionSequence`
    (:`then_0`
      (`KismetSystemLibrary.Delay` (`self.ActivationDelay`))
      (`PrimitiveComponent.SetCollisionEnabled` (`self.TriggerArea`) "QueryOnly"))
    (:`then_1`
      (if (not (`self.WasActivatedOnce`))
        (set `self.WasActivatedOnce` true)
        (`|ExecutionSequence`
          (:`then_0`
            (bind _returnvalue (`GameplayStatics.GetActorOfClass` "/Game/Blueprints/Props/BP_Door.BP_Door_C"))
            (`/Engine/EditorBlueprintResources/StandardMacros.IsValid` _returnvalue
              (:`Is Valid`
                (`/Game/Blueprints/Traps/BPI_TrapActivation.TrapActivated` _returnvalue))
              (:`Is Not Valid`
                _))
            (`self.TrapActivatedD`))
          (:`then_1`
            (bind _asbp_my_fall_gm (cast `/Game/Blueprints/BP_MyFallGM` (`GameplayStatics.GetGameMode`)))
            (`/Game/Blueprints/Traps/BPI_TrapActivation.TrapActivated` _asbp_my_fall_gm)))))))

(event `self.InteractionArea.OnComponentEndOverlap`
  (params (OverlappedComponent :type "PrimitiveComponent Object Reference") (OtherActor :type "Actor Object Reference") (OtherComp :type "PrimitiveComponent Object Reference") (OtherBodyIndex :type Integer))
  (bind _playerref (`self.PlayerRef`))
  ;[1 1 1] Interaction
  (if (== OtherActor (`GameplayStatics.GetPlayerCharacter` 0))
    (`/Engine/EditorBlueprintResources/StandardMacros.IsValid` _playerref
      (:`Is Valid`
        (set `/Game/Blueprints/Player/BP_Boris.AvailableInteractible` "NewEnumerator2" _playerref)
        (remove `/Game/Blueprints/Player/BP_Boris.Interact` _playerref (delegate `OnActivate`))))))

(event `self.TriggerArea.OnComponentBeginOverlap`
  (params (OverlappedComponent :type "PrimitiveComponent Object Reference") (OtherActor :type "Actor Object Reference") (OtherComp :type "PrimitiveComponent Object Reference") (OtherBodyIndex :type Integer) (bFromSweep :type Boolean) (SweepResult :type "HitResult Structure (by ref)"))
  ;[1 1 1] Triggering
  (if (`self.IsActive`)
    (bind _output_get (set `self.ActorThatOverlapsTrigger` OtherActor))
    (if (`self.ActorHasTag` _output_get "Player")
      (`self.TriggerOnPlayer`)
      (`self.Deactivate`)
      (`PrimitiveComponent.SetCollisionEnabled` (`self.TriggerArea`) "NoCollision")
      (elif (`self.ActorHasTag` _output_get "Enemy")
        (set `self.EnemyRef` _output_get)
        (`self.TriggerOnEnemy`)
        (`self.Deactivate`)
        (`PrimitiveComponent.SetCollisionEnabled` (`self.TriggerArea`) "NoCollision")
        (if (not (`self.WorkedOnEnemyAtLeastOnce`))
          (set `self.WorkedOnEnemyAtLeastOnce` true)
          (`self.TrapWorked`))))))

(event `self.TriggerArea.OnComponentEndOverlap`
  (params (OverlappedComponent :type "PrimitiveComponent Object Reference") (OtherActor :type "Actor Object Reference") (OtherComp :type "PrimitiveComponent Object Reference") (OtherBodyIndex :type Integer))
  ;[1 1 1] Triggering
  (set `self.ActorThatOverlapsTrigger` null)
  (set `self.EnemyRef` null))

(fn `Activate`
  (`self.EnableTrapMeshes`)
  (`self.DisableIndicator`)
  (set `self.IsActive` true))

(fn `Deactivate`
  (`self.EnableIndincator`)
  (`self.DisableTrapMeshes`)
  (set `self.IsActive` false))

(fn `DisableIndicator`
  (bind _interactionindicator (`self.InteractionIndicator`))
  (`PrimitiveComponent.SetCollisionEnabled` _interactionindicator "NoCollision")
  (`SceneComponent.SetVisibility` _interactionindicator false false))

(fn `DisableTrapMeshes`
  (for _array_element (`self.TrapMeshes`)
    (`PrimitiveComponent.SetCollisionEnabled` _array_element "NoCollision")
    (`SceneComponent.SetVisibility` _array_element false false)))

(fn `EnableIndincator`
  (bind _interactionindicator (`self.InteractionIndicator`))
  (`PrimitiveComponent.SetCollisionEnabled` _interactionindicator "QueryOnly")
  (`SceneComponent.SetVisibility` _interactionindicator true false))

(fn `EnableTrapMeshes`
  (for _array_element (`self.TrapMeshes`)
    (`PrimitiveComponent.SetCollisionEnabled` _array_element "QueryOnly")
    (`SceneComponent.SetVisibility` _array_element true false)))

(fn `TriggerOnEnemy`)

(fn `TriggerOnPlayer`)

(fn `UserConstructionScript`
  (`KismetArrayLibrary.Array_Add` (`self.TrapMeshes`) (`self.TrapMesh`)))