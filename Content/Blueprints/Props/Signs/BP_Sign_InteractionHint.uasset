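; Sign prop that shows a localized hint to hold the interaction key to set a trap.
; On BeginPlay it scans key mappings for the Interact input action and takes that key's long display name.
; It formats the name into hard-coded English and Russian strings, then calls AssignLocalizedText to apply them.
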(event `self.ReceiveBeginPlay`
  (bind _interactionkeyname (`self.InteractionKeyName`))
  (`parent.ReceiveBeginPlay`)
  (for _array_element (`self.Key Mappings`)
    (bind (_playermappableoptions _triggers _modifiers _action _key) (break `EnhancedActionKeyMapping` _array_element))
    (switch `string` (`KismetStringLibrary.Conv_NameToString` (`.Name` (break `PlayerMappableKeyOptions` _playermappableoptions)))
      (:`IAInteract`
        (set `self.InteractionKeyName` (`KismetTextLibrary.Conv_TextToString` (`KismetInputLibrary.Key_GetDisplayName` _key))))))
  (set `self.EnText` (`|FormatText` "Hold {E}  \nto set the trap" _interactionkeyname))
  (set `self.RuText` (`|FormatText` "Удерживать {E}, \nчтобы поставить ловушку" _interactionkeyname))
  (`self.AssignLocalizedText`))

(fn `UserConstructionScript`
  (`parent.UserConstructionScript`))