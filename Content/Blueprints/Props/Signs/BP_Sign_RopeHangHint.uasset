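; BP_Sign_RopeHangHint is a sign that shows a localized hint to hold the grab key mid-air to hang, presumably on ropes.
; On BeginPlay, after the parent's logic, it searches KeyMappings for the IA Grab action and reads that key's display name.
; It inserts the name into English and Russian text, then calls AssignLocalizedText, so the hint follows the mapped key instead of hardcoding it.
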(event `self.ReceiveBeginPlay`
  (bind _grabkeyname (`self.GrabKeyName`))
  (`parent.ReceiveBeginPlay`)
  (for _array_element (`self.Key Mappings`)
    (bind (_playermappableoptions _triggers _modifiers _action _key) (break `EnhancedActionKeyMapping` _array_element))
    (switch `string` (`KismetStringLibrary.Conv_NameToString` (`.Name` (break `PlayerMappableKeyOptions` _playermappableoptions)))
      (:`IAGrab`
        (set `self.GrabKeyName` (`KismetTextLibrary.Conv_TextToString` (`KismetInputLibrary.Key_GetDisplayName` _key))))))
  (set `self.EnText` (`|FormatText` "Hold  \n{LMB}  \nmid-air to hang" _grabkeyname))
  (set `self.RuText` (`|FormatText` "Удерживать  \n{LMB}, \nв воздухе, чтобы \nповиснуть" _grabkeyname))
  (`self.AssignLocalizedText`))

(fn `UserConstructionScript`
  (`parent.UserConstructionScript`))