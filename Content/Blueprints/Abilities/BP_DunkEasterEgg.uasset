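; Interactable basketball dunk easter egg that lets Boris, the player character, carry a ball that later returns to its starting spot.
; Overlapping the box offers the interaction and binds attach and detach events on Boris; leaving unbinds only the attach.
; Attaching snaps the ball to Boris's dunk socket and disables ball and hoop collision.
; Stopping the dunk restores collision and plays a timeline that lerps the ball back from its current location.
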(event `self.ReceiveBeginPlay`
  (set `self.DefaultBallLocation` (`SceneComponent.K2_GetComponentLocation` (`self.BallMesh`))))

(event `DetachBall`
  (bind _ballmesh (`self.BallMesh`))
  (`SceneComponent.K2_DetachFromComponent` (`self.BallMesh`) "KeepWorld" "KeepWorld" "KeepWorld" true)
  (`PrimitiveComponent.SetCollisionEnabled` (`self.BallMesh`) "QueryAndPhysics")
  (for _array_element (`|MakeArray` (`self.HoopMesh1`) (`self.HoopMesh2`) (`self.HoopMesh3`))
    (`PrimitiveComponent.SetCollisionEnabled` _array_element "QueryAndPhysics")
    (bind (_direction _alpha) (`Timeline|GetBallBack` :!via `PlayFromStart`)
      (:`Update`
        (`SceneComponent.K2_SetWorldLocation` _ballmesh (`KismetMathLibrary.VLerp` (`SceneComponent.K2_GetComponentLocation` _ballmesh) (`self.DefaultBallLocation`) _alpha) false false)))))

(event `self.Box.OnComponentBeginOverlap`
  (params (OverlappedComponent :type "PrimitiveComponent Object Reference") (OtherActor :type "Actor Object Reference") (OtherComp :type "PrimitiveComponent Object Reference") (OtherBodyIndex :type Integer) (bFromSweep :type Boolean) (SweepResult :type "HitResult Structure (by ref)"))
  (if (`self.ActorHasTag` OtherActor "Player")
    (bind _asbp_boris (cast `/Game/Blueprints/Player/BP_Boris` OtherActor))
    (set `/Game/Blueprints/Player/BP_Boris.AvailableInteractible` "NewEnumerator3" _asbp_boris)
    (add `/Game/Blueprints/Player/BP_Boris.Interact` _asbp_boris (delegate `AttachBall`))
    (add `/Game/Blueprints/Player/BP_Boris.StopDunk` _asbp_boris (delegate `DetachBall`))
    (set `/Game/Blueprints/Player/BP_Boris.DunkEERef` self _asbp_boris)))

(event `AttachBall`
  (`SceneComponent.K2_AttachToComponent` (`self.BallMesh`) (`/Game/Blueprints/Player/BP_Boris.DunkEasterEggSocket` (stale `self.Box.OnComponentBeginOverlap` _asbp_boris)) "None" "SnapToTarget" "KeepWorld" "KeepWorld" true)
  (`PrimitiveComponent.SetCollisionEnabled` (`self.BallMesh`) "NoCollision")
  (for _array_element (`|MakeArray` (`self.HoopMesh1`) (`self.HoopMesh2`) (`self.HoopMesh3`))
    (`PrimitiveComponent.SetCollisionEnabled` _array_element "NoCollision")))

(event `self.Box.OnComponentEndOverlap`
  (params (OverlappedComponent :type "PrimitiveComponent Object Reference") (OtherActor :type "Actor Object Reference") (OtherComp :type "PrimitiveComponent Object Reference") (OtherBodyIndex :type Integer))
  (if (`self.ActorHasTag` OtherActor "Player")
    (bind _asbp_boris (cast `/Game/Blueprints/Player/BP_Boris` OtherActor))
    (set `/Game/Blueprints/Player/BP_Boris.AvailableInteractible` "NewEnumerator2" _asbp_boris)
    (remove `/Game/Blueprints/Player/BP_Boris.Interact` _asbp_boris (delegate `AttachBall`))
    (`PrimitiveComponent.SetCollisionEnabled` (`self.BallMesh`) "QueryAndPhysics")))

(fn `UserConstructionScript`)