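; A pressure-button moving platform that shifts between default and activated positions while Player, Enemy or Small tagged actors stand in its trigger box.
; Overlaps update an object counter, and a DoOnce starts two timelines that lerp the button and platform meshes.
; When the count empties, a short delayed recheck guards against a bug before reversing both timelines and resetting the DoOnce.
; An elevator sound spawned at BeginPlay is unpaused during platform movement.
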(event `self.ReceiveBeginPlay`
  (bind _returnvalue (`GameplayStatics.SpawnSoundAtLocation` "/Game/SFX/GameplayEffects/Puzzle/Elevator.Elevator" (`SceneComponent.K2_GetComponentLocation` (`self.PlatformMesh`)) (struct) 1.0 1.0 0.0 "/Game/SFX/Soundtracks/SA_Music.SA_Music" "/Game/SFX/SoundConcurrency.SoundConcurrency"))
  (bind _output_get (set `self.SoundComponent` _returnvalue))
  (`AudioComponent.SetPaused` _output_get true))

(event `self.BoxCollision.OnComponentBeginOverlap`
  (params (OverlappedComponent :type "PrimitiveComponent Object Reference") (OtherActor :type "Actor Object Reference") (OtherComp :type "PrimitiveComponent Object Reference") (OtherBodyIndex :type Integer) (bFromSweep :type Boolean) (SweepResult :type "HitResult Structure (by ref)"))
  (if (or (`self.ActorHasTag` OtherActor "Player") (`self.ActorHasTag` OtherActor "Enemy") (`self.ActorHasTag` OtherActor "Small"))
    (bind _result (`/Engine/EditorBlueprintResources/StandardMacros.IncrementInt` (`self.CollidingObjects`))
      (:`  `
        (if (> _result 0)
          (`/Engine/EditorBlueprintResources/StandardMacros.DoOnce` false :!label _label
            (:`Completed`
              (`|ExecutionSequence`
                (:`then_0`
                  (bind (_direction _pushstate) (`Timeline|Timeline` :!label _label_2)
                    (:`Update`
                      (`SceneComponent.K2_SetRelativeLocation` (`self.ButtonMesh`) (`KismetMathLibrary.VLerp` (0.0 0.0 0.0) (`self.ActiveButtonPos`) _pushstate) false false))))
                (:`then_1`
                  (bind (_direction_2 _pushstate_2) (`Timeline|Timeline_0` :!label _label_3)
                    (:`Update`
                      (`SceneComponent.K2_SetRelativeLocation` (`self.PlatformMesh`) (`KismetMathLibrary.VLerp` (`self.PlatformDefaultRelativeLocation`) (`self.PlatformActivatedtRelativeLocation`) _pushstate_2) false false)
                      (`AudioComponent.SetPaused` (`self.SoundComponent`) false))
                    (:`Finished`
                      (`AudioComponent.SetPaused` (`self.SoundComponent`) true))))))))))))

(event `self.BoxCollision.OnComponentEndOverlap`
  (params (OverlappedComponent :type "PrimitiveComponent Object Reference") (OtherActor :type "Actor Object Reference") (OtherComp :type "PrimitiveComponent Object Reference") (OtherBodyIndex :type Integer))
  (if (or (`self.ActorHasTag` OtherActor "Player") (`self.ActorHasTag` OtherActor "Enemy") (`self.ActorHasTag` OtherActor "Small"))
    (bind _result (`/Engine/EditorBlueprintResources/StandardMacros.DecrementInt` (`self.CollidingObjects`))
      (:`  `
        (if (<= (`KismetMathLibrary.Clamp` _result 0 10) 0)
          ;[1 1 1] After delay additional branch to prevent bug
          (`KismetSystemLibrary.Delay` 0.5)
          (if (<= (`self.CollidingObjects`) 0)
            (`|ExecutionSequence`
              (:`then_0`
                (goto _label_2 :!via `Reverse`))
              (:`then_1`
                (goto _label_3 :!via `Reverse`))
              (:`then_2`
                (goto _label :!via `Reset`)))))))))

(fn `UserConstructionScript`)