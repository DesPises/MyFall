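; Pie trap Blueprint that swings a temporary pie mesh when triggered by the player or an enemy.
; Both triggers rotate the actor from the overlapping actor's right vector, then a timeline rolls the spawned mesh 90 degrees before destroying it.
; Player triggers call GetTrappedByPie when the animation finishes.
; Enemy triggers instead set the TrapType blackboard key before the animation starts.
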(event `self.TriggerOnPlayer`
  ;[1 1 1] Trigger
  (set `self.ActivatedByPlayer` true)
  (`self.K2_SetActorRotation` (`KismetMathLibrary.Conv_VectorToRotator` (* (`self.GetActorRightVector` (`self.ActorThatOverlapsTrigger`)) -1.0)) :!label _label)
  (bind _returnvalue (`AddComponent|NODE_AddStaticMeshComponent-0`))
  (`StaticMeshComponent.SetStaticMesh` _returnvalue "/Game/3D/Traps/Pie/PieTrap.PieTrap")
  (bind (_direction _alpha) (`Timeline|Animation` :!via `PlayFromStart`)
    (:`Update`
      (`SceneComponent.K2_SetRelativeRotation` _returnvalue (`KismetMathLibrary.MakeRotator` (`KismetMathLibrary.Lerp` 0.0 -90.0 _alpha)) false false))
    (:`Finished`
      (if (`self.ActivatedByPlayer`)
        (`/Game/Blueprints/Player/BP_Boris.GetTrappedByPie` (`self.PlayerRef`)))
      (`ActorComponent.K2_DestroyComponent` _returnvalue))))

(event `self.TriggerOnEnemy`
  ;[1 1 1] Trigger
  (bind _asbp_enemy (cast `/Game/Blueprints/Enemies/BP_Enemy` (`self.EnemyRef`)))
  (`BlackboardComponent.SetValueAsEnum` (`AIBlueprintHelperLibrary.GetBlackboard` _asbp_enemy) "TrapType" 3)
  (set `self.ActivatedByPlayer` false)
  (goto _label))

(fn `UserConstructionScript`
  (`parent.UserConstructionScript`))